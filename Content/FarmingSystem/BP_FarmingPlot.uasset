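; BP_FarmingPlot is a farming plot actor that snaps pickable items onto it and handles crop planting.
; On BeginPlay it takes the class of its parent BP_MasterSeed actor as the plant to spawn.
; A box overlap moves the first FarmingInterface actor tagged Pickable to the arrow's location, gated by DoOnce.
; PlantCrop spawns that class ahead of the player at fixed height, owned by a debug-drawn trace's hit actor, and returns false.
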(event `self.ReceiveBeginPlay`
  (bind _asbp_master_seed (cast `/Game/FarmingSystem/BP_MasterSeed` (`self.GetParentActor`)))
  (bind _output_get (set `self.As BP Master Seed` _asbp_master_seed))
  (set `self.Plant` (`GameplayStatics.GetObjectClass` _output_get)))

(event `self.Box.OnComponentBeginOverlap`
  (params (OverlappedComponent :type "PrimitiveComponent Object Reference") (OtherActor :type "Actor Object Reference") (OtherComp :type "PrimitiveComponent Object Reference") (OtherBodyIndex :type Integer) (bFromSweep :type Boolean) (SweepResult :type "HitResult Structure (by ref)"))
  (if (and (`KismetSystemLibrary.DoesImplementInterface` OtherActor "/Game/FarmingSystem/FarmingInterface.FarmingInterface_C") (`self.ActorHasTag` OtherActor "Pickable"))
    (`/Engine/EditorBlueprintResources/StandardMacros.DoOnce` false
      (:`Completed`
        (`self.K2_SetActorLocation` OtherActor (`SceneComponent.K2_GetComponentLocation` (`self.Arrow`)) false false)))))

(fn `PlantCrop`
  (params (Playyer :type "Actor Object Reference"))
  (returns (NewParam :type Boolean))
  (bind _returnvalue (`self.K2_GetActorRotation` Playyer))
  (bind (_returnvalue_x _returnvalue_y _returnvalue_z) (`KismetMathLibrary.BreakVector` (+ (`self.K2_GetActorLocation` Playyer) (* (`KismetMathLibrary.GetForwardVector` _returnvalue) 500.0))))
  (set `self.Playyer` Playyer)
  (bind _outhit (`KismetSystemLibrary.LineTraceSingle` :`End` (`KismetMathLibrary.MakeVector` _returnvalue_x _returnvalue_y _returnvalue_z) :`TraceChannel` "TraceTypeQuery1" :`DrawDebugType` "ForDuration"))
  (`|SpawnActorFromClass` (`self.Plant`) (`KismetMathLibrary.MakeTransform` (`KismetMathLibrary.MakeVector` _returnvalue_x _returnvalue_y 20.0) (`KismetMathLibrary.MakeRotator` (.roll _returnvalue) 0.0 (.yaw _returnvalue))) "Undefined" "MultiplyWithRoot" (`.HitActor` (`GameplayStatics.BreakHitResult` _outhit)) null)
  (return false))

(fn `UserConstructionScript`)