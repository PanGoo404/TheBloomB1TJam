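; BP_TopCap is a procedural-generation cap piece that swaps overlapping actors for end caps and can be recolored.
; When its Box begins an overlap and that overlapped component carries the "Door" tag, it always spawns BP_EndCap at the other actor's transform and destroys that actor.
; The SendColorVector event creates a dynamic material instance from the Cube's material to set its base color.
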(event `self.Box.OnComponentBeginOverlap`
  (params (OverlappedComponent :type "PrimitiveComponent Object Reference") (OtherActor :type "Actor Object Reference") (OtherComp :type "PrimitiveComponent Object Reference") (OtherBodyIndex :type Integer) (bFromSweep :type Boolean) (SweepResult :type "HitResult Structure (by ref)"))
  (if (`ActorComponent.ComponentHasTag` OverlappedComponent "Door")
    (if true
      (`|SpawnActorFromClass` "/Game/Procedural/EndCap/BP_EndCap.BP_EndCap_C" (`self.GetTransform` OtherActor) "AlwaysSpawn" "MultiplyWithRoot" null null))
    (`self.K2_DestroyActor` OtherActor)))

(event `/Game/Procedural/Interfaces/BI_RandomDataParser.SendColorVector`
  (params (Color :type "Vector Structure"))
  (bind _cube (`self.Cube`))
  (bind _returnvalue (`KismetMaterialLibrary.CreateDynamicMaterialInstance` (`PrimitiveComponent.GetMaterial` _cube 0)))
  (`MaterialInstanceDynamic.SetVectorParameterValue` _returnvalue "Base Color" (`KismetMathLibrary.Conv_VectorToLinearColor` Color))
  (`PrimitiveComponent.SetMaterial` _cube 0 null))

(fn `UserConstructionScript`)