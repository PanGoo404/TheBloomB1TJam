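; Base room actor for procedural level generation that tints its walls a random color and spawns an actor at each exit.
; Each exit picks one of two EndCaps classes by a random roll using remaining room budget and PriorityID, then passes the color to the spawn.
; PriorityID is the construction time in whole seconds, so on overlap of a "Room"-tagged component the room destroys itself if the other actor's ID is lower.
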(event `self.ReceiveBeginPlay`
  ; Randomize Color and propagate
  (bind _output_get (set `self.Color` (+ (* (`KismetMathLibrary.RandomUnitVector`) (0.8 0.8 0.8)) (1.0 1.0 1.0))))
  (for _array_element (`SceneComponent.GetChildrenComponents` (`self.Walls`) false)
    (bind _asstatic_mesh_component (cast `StaticMeshComponent` _array_element))
    (bind _returnvalue (`KismetMaterialLibrary.CreateDynamicMaterialInstance` (`PrimitiveComponent.GetMaterial` _asstatic_mesh_component 0)))
    (`MaterialInstanceDynamic.SetVectorParameterValue` _returnvalue "Base Color" (`KismetMathLibrary.Conv_VectorToLinearColor` _output_get))
    (`PrimitiveComponent.SetMaterial` _asstatic_mesh_component 0 _returnvalue))
  ; Fill Entry points
  (for _array_element_2 (`SceneComponent.GetChildrenComponents` (`self.Exits`) false)
    ; Noodle randomizer
    (bind _outactors (`GameplayStatics.GetAllActorsOfClass` "BP_MasterRoom_Base_C"))
    (bind _returnvalue_2 (`KismetArrayLibrary.Array_Length` _outactors))
    (bind _returnvalue_3 (`KismetMathLibrary.RandomInteger` (- (`self.Max expected rooms`) _returnvalue_2)))
    (bind _returnvalue_4 (`KismetMathLibrary.Conv_BoolToInt` (< _returnvalue_3 (mod (`self.PriorityID`) 60))))
    (`KismetSystemLibrary.PrintText` (`|FormatText` "NoR: {NOR} SEED: {SS} Pick: {ClassID}" _returnvalue_2 _returnvalue_3 _returnvalue_4))
    (bind _output (`|GetArrayItem` (`self.EndCaps`) _returnvalue_4))
    (bind _returnvalue_5 (`KismetSystemLibrary.GetClassDisplayName` _output))
    (`KismetSystemLibrary.PrintText` (`|FormatText` "Picked {Entity}" _returnvalue_5))
    (bind _returnvalue_6 (`|SpawnActorFromClass` _output (`SceneComponent.K2_GetComponentToWorld` _array_element_2) "AlwaysSpawn" "MultiplyWithRoot" null null))
    (`KismetArrayLibrary.Array_Add` (`self.Doors`) _returnvalue_6)
    (if (`KismetSystemLibrary.IsValid` _returnvalue_6)
      (message `/Game/Procedural/Interfaces/BI_RandomDataParser.SendColorVector` _returnvalue_6 _output_get)
      (`KismetSystemLibrary.PrintText` (`|FormatText` "Spawned {Entity}" _returnvalue_5)))))

(event `self.Overlapper.OnComponentBeginOverlap`
  (params (OverlappedComponent :type "PrimitiveComponent Object Reference") (OtherActor :type "Actor Object Reference") (OtherComp :type "PrimitiveComponent Object Reference") (OtherBodyIndex :type Integer) (bFromSweep :type Boolean) (SweepResult :type "HitResult Structure (by ref)"))
  ; Overlapper
  (if (and (`KismetSystemLibrary.IsValid` OtherActor) (`ActorComponent.ComponentHasTag` OverlappedComponent "Room"))
    (bind _outputid (message `/Game/Procedural/Interfaces/BI_IDPasser.GetID` OtherActor 0))
    (if (> (`self.PriorityID`) _outputid)
      (`self.K2_DestroyActor`))))

(fn `GetID`
  (params (InputID :type Integer))
  (returns (OutputID :type Integer))
  (return (`self.PriorityID`)))

(fn `UserConstructionScript`
  (set `self.PriorityID` (`KismetMathLibrary.FTrunc` (`GameplayStatics.GetTimeSeconds`))))