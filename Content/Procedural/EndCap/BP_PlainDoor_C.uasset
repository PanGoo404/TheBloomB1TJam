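; Plain door Blueprint in the procedural end-cap set, printing a "substituted" debug message on BeginPlay.
; Interact alternates between Open and Close through a FlipFlop.
; When its Overlapper component begins an overlap, it destroys the other actor if the Overlapper itself carries the PlainDoor tag, with no check on that actor.
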(event `self.ReceiveBeginPlay`
  (`parent.ReceiveBeginPlay`)
  (`KismetSystemLibrary.PrintText` "Plain door  : Substituted"))

(event `/Game/Procedural/Interfaces/BI_Interactable.Interact`
  (`/Engine/EditorBlueprintResources/StandardMacros.FlipFlop`
    (:`A`
      (`self.Open`))
    (:`B`
      (`self.Close`))))

(event `self.Overlapper.OnComponentBeginOverlap`
  (params (OverlappedComponent :type "PrimitiveComponent Object Reference") (OtherActor :type "Actor Object Reference") (OtherComp :type "PrimitiveComponent Object Reference") (OtherBodyIndex :type Integer) (bFromSweep :type Boolean) (SweepResult :type "HitResult Structure (by ref)"))
  (if (`ActorComponent.ComponentHasTag` OverlappedComponent "PlainDoor")
    (`self.K2_DestroyActor` OtherActor)))

(fn `UserConstructionScript`
  (`parent.UserConstructionScript`))