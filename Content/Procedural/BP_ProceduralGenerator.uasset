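; BP_ProceduralGenerator is a procedural generator actor that spawns the starting BP_Elevator at its root transform on BeginPlay.
; BeginPlay also totals the float keys of the Class map into Weight and copies them to RefSortedKeys, after the descending sort call.
; GenerateEndPoint returns the first class whose key is within a random roll up to Weight, lowered by NumberOfDoors over a random divisor.
; Door spawning at elevator exits is unconnected.
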(event `SpawnStart`
  (bind (_returnvalue_location _returnvalue_rotation _returnvalue_scale) (`KismetMathLibrary.BreakTransform` (`SceneComponent.K2_GetComponentToWorld` (`self.DefaultSceneRoot`))))
  ; Spawn
  (bind _returnvalue (`|SpawnActorFromClass` "/Game/Procedural/Rooms/BP_Elevator.BP_Elevator_C" (`KismetMathLibrary.MakeTransform` _returnvalue_location _returnvalue_rotation _returnvalue_scale) "AlwaysSpawn" "MultiplyWithRoot" null null)))

(event `self.ReceiveBeginPlay`
  (`KismetSystemLibrary.PrintText` (`|FormatText` "Gen object call : {call}" (`KismetSystemLibrary.GetObjectName` self)))
  (bind _keys (`BlueprintMapLibrary.Map_Keys` (`self.Class`)))
  (`KismetArrayLibrary.SortFloatArray` (stale _output_get) false "Descending")
  (for _array_element _keys
    (set `self.Weight` (+ _array_element (`self.Weight`)))
    (bind _output_get (set `self.RefSortedKeys` _keys)))
  (`self.SpawnStart`)
  (`KismetSystemLibrary.PrintText` (`|FormatText` "Prepared to spawn Elevator: {call}" (`KismetSystemLibrary.GetObjectName` self))))

(fn `GenerateEndPoint`
  (returns (PickedClass :type "Actor Class Reference"))
  (bind _returnvalue (- (`KismetMathLibrary.RandomInteger` (`KismetMathLibrary.Round` (`self.Weight`))) (/ (`self.NumberOfDoors`) (`KismetMathLibrary.RandomInteger` 3))))
  (for _array_element (`self.RefSortedKeys`)
    (if (<= _array_element _returnvalue)
      (bind _value (`BlueprintMapLibrary.Map_Find` (`self.Class`) _array_element))
      (`KismetSystemLibrary.PrintText` (`|FormatText` "Randomiser : {Number} Picked class : {Class}" _returnvalue (`KismetSystemLibrary.GetClassDisplayName` _value)))
      (return _value))))

(fn `UserConstructionScript`)