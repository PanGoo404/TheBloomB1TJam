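; Procedural mine room that populates itself with randomly chosen points of interest (POIs) when play begins.
; Each child component of SpawnPoints gets an actor spawned at its location, with a randomized rotation.
; PickRandomPOI makes a weighted pick, rolling against TotalBase and walking cumulative probabilities in POIList to return a class.
; Its debug print re-rolls the random values, so the shown number differs from the actual pick.
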(event `self.ReceiveBeginPlay`
  (`parent.ReceiveBeginPlay`)
  ; Loop through spawn points
  (for _array_element (`SceneComponent.GetChildrenComponents` (`self.SpawnPoints`) false)
    ; Compacted version with float pick
    (bind _pickedpoi (`self.PickRandomPOI`))
    (bind (_returnvalue_location _returnvalue_rotation) (`KismetMathLibrary.BreakTransform` (`SceneComponent.K2_GetComponentToWorld` _array_element)))
    (`|SpawnActorFromClass` _pickedpoi (`KismetMathLibrary.MakeTransform` _returnvalue_location (`KismetMathLibrary.Conv_VectorToRotator` (* (`KismetMathLibrary.RandomUnitVector`) _returnvalue_rotation))) "Undefined" "MultiplyWithRoot" null null)))

(fn `PickRandomPOI`
  (returns (PickedPOI :type "Actor Class Reference"))
  (locals (Base :type "Float (double-precision)") (`Current Pick` :type "Float (double-precision)"))
  (bind _base (`local.Base`))
  (bind _totalbase (`self.TotalBase`))
  (bind _returnvalue (`KismetMathLibrary.RandomInteger` (- (`KismetMathLibrary.FTrunc` _totalbase) 1)))
  (bind _returnvalue_2 (+ (`KismetMathLibrary.RandomFloat`) _returnvalue))
  (bind _output_get (set `local.Current Pick` _returnvalue_2))
  ; Pick a POI
  (for _array_element (`self.POIList`)
    (bind (_poisclass _poisprobability) (break `/Game/Procedural/Structs/BS_POI+Prob` _array_element))
    (bind _returnvalue_3 (+ _base _poisprobability))
    (if (and (<= _output_get _returnvalue_3) (> _output_get _base))
      (`KismetSystemLibrary.PrintText` (`|FormatText` "Random number: {RN}({Raw})/{Base} Picked{Pick}" _returnvalue_2 _returnvalue _totalbase _poisprobability))
      (set `local.Base` 0.0)
      (return _poisclass)
      (else
        (set `local.Base` _returnvalue_3))))
  (return null))

(fn `UserConstructionScript`
  (`parent.UserConstructionScript`))