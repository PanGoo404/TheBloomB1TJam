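; BP_MasterSeed is a farming seed that plants itself on overlap with a FarmingInterface actor and grows through three mesh stages.
; A one-time overlap snaps it to that actor and stops Sphere1's physics, then chained timelines scale the sphere and swap StaticMesh, printing debug values.
; An alternative timer-driven stage chain exists, but its starting branch is disconnected.
; PlantCrop is a stub returning false.
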(event `FirstGrowthStage`
  (`StaticMeshComponent.SetStaticMesh` (`self.StaticMesh`) (`self.FirstStageMesh`))
  (`KismetSystemLibrary.K2_SetTimerDelegate` (delegate `SecondGrowthStage`) (`self.StageGrowthTime2`) false true)
  (bind (_direction _newtrack_0) (`Timeline|Oś czasu`)
    (:`Update`
      (bind _returnvalue (`KismetMathLibrary.Lerp` 0.1 (`self.GrowthScaleTreshold_1`) _newtrack_0))
      (`SceneComponent.SetWorldScale3D` (`self.Sphere1`) (`KismetMathLibrary.Conv_DoubleToVector` _returnvalue))
      (`KismetSystemLibrary.PrintText` (`KismetTextLibrary.Conv_DoubleToText` _returnvalue "HalfToEven")))))

(event `self.Sphere1.OnComponentBeginOverlap`
  (params (OverlappedComponent :type "PrimitiveComponent Object Reference") (OtherActor :type "Actor Object Reference") (OtherComp :type "PrimitiveComponent Object Reference") (OtherBodyIndex :type Integer) (bFromSweep :type Boolean) (SweepResult :type "HitResult Structure (by ref)"))
  (bind _staticmesh (`self.StaticMesh`))
  (bind _growthscaletreshold_1 (`self.GrowthScaleTreshold_1`))
  (bind _growthscaletreshold_2 (`self.GrowthScaleTreshold_2`))
  (if (`KismetSystemLibrary.DoesImplementInterface` OtherActor "/Game/FarmingSystem/FarmingInterface.FarmingInterface_C")
    (`/Engine/EditorBlueprintResources/StandardMacros.DoOnce` false
      (:`Completed`
        (`SceneComponent.K2_SetWorldLocation` (`self.DefaultSceneRoot`) (- (`self.K2_GetActorLocation` OtherActor) (0.0 0.0 0.0)) false true)
        (`SceneComponent.K2_SetRelativeRotation` :`self` (`self.Sphere1`))
        (`PrimitiveComponent.SetSimulatePhysics` (`self.Sphere1`) false)
        (`KismetSystemLibrary.PrintText` "Wairant 2")
        (`StaticMeshComponent.SetStaticMesh` _staticmesh (`self.FirstStageMesh`))
        (bind (_direction _newtrack_0) (`Timeline|Oś czasu_2`)
          (:`Update`
            (bind _returnvalue (`KismetMathLibrary.Lerp` 0.1 _growthscaletreshold_1 _newtrack_0))
            (`SceneComponent.SetWorldScale3D` (`self.Sphere1`) (`KismetMathLibrary.Conv_DoubleToVector` _returnvalue))
            (`KismetSystemLibrary.PrintText` (`KismetTextLibrary.Conv_DoubleToText` _returnvalue "HalfToEven")))
          (:`Finished`
            (`StaticMeshComponent.SetStaticMesh` _staticmesh (`self.SecondStageMesh`))
            (`KismetSystemLibrary.K2_SetTimerDelegate` :`Time` (`self.StageGrowthTime3`) :`bMaxOncePerFrame` true)
            (bind (_direction_2 _newtrack_0_2) (`Timeline|Oś czasu_3`)
              (:`Update`
                (bind _returnvalue_2 (`KismetMathLibrary.Lerp` _growthscaletreshold_1 _growthscaletreshold_2 _newtrack_0_2))
                (`SceneComponent.SetWorldScale3D` (`self.Sphere1`) (`KismetMathLibrary.Conv_DoubleToVector` _returnvalue_2))
                (`KismetSystemLibrary.PrintText` (`KismetTextLibrary.Conv_DoubleToText` _returnvalue_2 "HalfToEven")))
              (:`Finished`
                (`StaticMeshComponent.SetStaticMesh` _staticmesh (`self.FinalStageMesh`))
                (bind (_direction_3 _newtrack_0_3) (`Timeline|Oś czasu_4`)
                  (:`Update`
                    (bind _returnvalue_3 (`KismetMathLibrary.Lerp` _growthscaletreshold_2 0.5 _newtrack_0_3))
                    (`SceneComponent.SetWorldScale3D` (`self.Sphere1`) (`KismetMathLibrary.Conv_DoubleToVector` _returnvalue_3))
                    (`KismetSystemLibrary.PrintText` (`KismetTextLibrary.Conv_DoubleToText` _returnvalue_3 "HalfToEven"))))))))))))

(event `SecondGrowthStage`
  (`StaticMeshComponent.SetStaticMesh` (`self.StaticMesh`) (`self.SecondStageMesh`))
  (`KismetSystemLibrary.K2_SetTimerDelegate` (delegate `FinalGrowthStage`) (`self.StageGrowthTime3`) false true)
  (bind (_direction _newtrack_0) (`Timeline|Oś czasu_0`)
    (:`Update`
      (bind _returnvalue (`KismetMathLibrary.Lerp` (`self.GrowthScaleTreshold_1`) (`self.GrowthScaleTreshold_2`) _newtrack_0))
      (`SceneComponent.SetWorldScale3D` (`self.Sphere1`) (`KismetMathLibrary.Conv_DoubleToVector` _returnvalue))
      (`KismetSystemLibrary.PrintText` (`KismetTextLibrary.Conv_DoubleToText` _returnvalue "HalfToEven")))))

(event `FinalGrowthStage`
  (bind (_direction _newtrack_0) (`Timeline|Oś czasu_1`)
    (:`Update`
      (bind _returnvalue (`KismetMathLibrary.Lerp` (`self.GrowthScaleTreshold_2`) 0.5 _newtrack_0))
      (`SceneComponent.SetWorldScale3D` (`self.Sphere1`) (`KismetMathLibrary.Conv_DoubleToVector` _returnvalue)))
    (:`Finished`
      (`StaticMeshComponent.SetStaticMesh` (`self.StaticMesh`) (`self.FinalStageMesh`))
      (`KismetSystemLibrary.PrintText` (`KismetTextLibrary.Conv_DoubleToText` _returnvalue "HalfToEven")))))

(fn `PlantCrop`
  (params (Playyer :type "Actor Object Reference"))
  (returns (NewParam :type Boolean))
  (return false))

(fn `UserConstructionScript`)