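; Procedural generation door that, on first interaction, spawns a random room from RoomClasses, with rare altar or emergency elevator rolls, then toggles open and closed.
; A timeline swings the Axis yaw, and AI can only open doors already used.
; Overlaps tagged Door or Walls compare construction-time PriorityIDs to remove the door or replace it with a plain door or end cap.
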(event `/Game/Procedural/Interfaces/BI_Interactable.Interact`
  ; Interaction
  (if (`self.WasUsed?`)
    (if (`self.IsOpen?`)
      (`self.Close`)
      (set `self.IsOpen?` false)
      (else
        (`self.Open`)
        (set `self.IsOpen?` true :!label _label)))
    (else
      (`/Engine/EditorBlueprintResources/StandardMacros.DoOnce` false
        (:`Completed`
          (`self.SpawnNextRoom`)
          (set `self.WasUsed?` true)
          (`self.Open`)
          (goto _label))))))

(event `Open`
  ; animation control
  (bind (_direction _door) (`Timeline|Opening Animation` :!label _label_2)
    (:`Update`
      (`SceneComponent.K2_SetRelativeRotation` (`self.Axis`) (`KismetMathLibrary.MakeRotator` 0.0 0.0 (`KismetMathLibrary.Lerp` 0.0 (`self.Opened Angle`) _door)) false false))))

(event `Close`
  ; animation control
  (goto _label_2 :!via `Reverse`))

(event `/Game/Procedural/Interfaces/BI_AIInteract.AIOpen`
  ; AI Handling
  (if (`self.IsOpen?`)
    _
    (elif (`self.WasUsed?`)
      (`self.Open`)
      (set `self.IsOpen?` true))))

(event `/Game/Procedural/Interfaces/BI_AIInteract.AIClose`
  ; AI Handling
  (if (`self.IsOpen?`)
    (`self.Close`)
    (set `self.IsOpen?` false)))

(event `self.Overlapper.OnComponentBeginOverlap`
  (params (OverlappedComponent :type "PrimitiveComponent Object Reference") (OtherActor :type "Actor Object Reference") (OtherComp :type "PrimitiveComponent Object Reference") (OtherBodyIndex :type Integer) (bFromSweep :type Boolean) (SweepResult :type "HitResult Structure (by ref)"))
  ; Handle Collision with doors
  (if (`ActorComponent.ComponentHasTag` OverlappedComponent "Door")
    ; Validation
    (if (`KismetSystemLibrary.IsValid` OtherActor)
      (bind _outputid (message `/Game/Procedural/Interfaces/BI_IDPasser.GetID` OtherActor 0))
      (if (> (`self.PriorityID`) _outputid)
        (`self.K2_DestroyActor`)
        (else
          (`|SpawnActorFromClass` "/Game/Procedural/EndCap/BP_PlainDoor_C.BP_PlainDoor_C_C" (`SceneComponent.GetRelativeTransform` (`self.DefaultSceneRoot`)) "AlwaysSpawn" "OverrideRootScale" null null)
          (`self.K2_DestroyActor`))))
    (else
      ; Handle Wall Collision
      (if (`ActorComponent.ComponentHasTag` OverlappedComponent "Walls")
        (bind _outputid_2 (message `/Game/Procedural/Interfaces/BI_IDPasser.GetID` OtherActor 0))
        (if (> (`self.PriorityID`) _outputid_2)
          (`|SpawnActorFromClass` "/Game/Procedural/EndCap/BP_EndCap.BP_EndCap_C" (`SceneComponent.GetRelativeTransform` (`self.DefaultSceneRoot`)) "AlwaysSpawn" "OverrideRootScale" null null)
          (`self.K2_DestroyActor`)
          (else
            ;; Jestem drzwiami starymi
            (`|SpawnActorFromClass` "/Game/Procedural/EndCap/BP_PlainDoor_C.BP_PlainDoor_C_C" (`SceneComponent.GetRelativeTransform` (`self.DefaultSceneRoot`)) "AlwaysSpawn" "OverrideRootScale" null null)
            (`self.K2_DestroyActor`)))
        (else
          ; Un Handled Exeption throw
          (`KismetSystemLibrary.PrintString` (`KismetSystemLibrary.GetDisplayName` OverlappedComponent)))))))

(event `self.ReceiveBeginPlay`
  ; Overlapper and init
  (`TimelineComponent.SetPlayRate` (`self.Opening Animation`) (`self.Duration`)))

(fn `GetID`
  (params (InputID :type Integer))
  (returns (OutputID :type Integer))
  (return (`self.PriorityID`)))

(fn `SpawnNextRoom`
  (bind (_returnvalue_location _returnvalue_rotation) (`KismetMathLibrary.BreakTransform` (`SceneComponent.K2_GetComponentToWorld` (`self.DefaultSceneRoot`))))
  (if (== (`KismetMathLibrary.RandomInteger` 50) 35)
    (set `self.pom` "/Game/Procedural/Rooms/BP_Altar.BP_Altar_C")
    (elif (== (`KismetMathLibrary.RandomInteger` 40) 30)
      (bind _output_get (set `self.pom` "/Game/Procedural/Rooms/BP_ElevatorEmergency.BP_ElevatorEmergency_C"))
      (else
        (set `self.pom` (`KismetArrayLibrary.Array_Random` (`self.RoomClasses`))))))
  (`|SpawnActorFromClass` _output_get (`KismetMathLibrary.MakeTransform` _returnvalue_location _returnvalue_rotation) "AlwaysSpawn" "MultiplyWithRoot" null null)
  ; Debbug
  (`KismetSystemLibrary.PrintText` (`|FormatText` "Pojawiło się pomieszcznie : {Lokazlizacja}" (`KismetStringLibrary.Conv_VectorToString` _returnvalue_location)))
  (`KismetSystemLibrary.PrintText` (`|FormatText` (`KismetTextLibrary.Conv_StringToText` (`KismetStringLibrary.Conv_VectorToString` (+ (`SceneComponent.RelativeLocation` (`self.DefaultSceneRoot`)) _returnvalue_location))))))

(fn `UserConstructionScript`
  (bind _output_get (set `self.PriorityID` (`KismetMathLibrary.FTrunc` (`GameplayStatics.GetTimeSeconds`))))
  (`KismetSystemLibrary.PrintText` (`|FormatText` "Assigned door ID : {Assigned ID}" _output_get)))